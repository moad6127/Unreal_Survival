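; BP_InteractLocation_Chest is an interactable chest actor that shows an interact prompt and opens a dual-inventory screen.
; ShowInteractPrompt writes the InteractText into the WBP_CanInteract_Button hosted by its widget component, then runs the parent's prompt logic.
; OnShowDualInventory creates a WBP_ChestInventory for the owning controller, passing the source inventory as player and target as chest, stores it and adds it to the viewport.
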(event `CanInteractInterface.ShowInteractPrompt`
  (bind _aswbp_can_interact_button (cast `/Game/Survival/UI/InteractWidgets/CanInteract/WBP_CanInteract_Button` (`WidgetComponent.GetUserWidgetObject` (`self.InteractWidgetComponent`))))
  (set `/Game/Survival/UI/InteractWidgets/CanInteract/WBP_CanInteract_Button.InteractText` (`self.InteractText`) _aswbp_can_interact_button)
  (`parent.ShowInteractPrompt`))

(event `self.OnShowDualInventory`
  (params (OwningController :type "PlayerController Object Reference") (SourceInventory :type "ExtenedInventoryComponent Object Reference") (TargetInventory :type "ExtenedInventoryComponent Object Reference"))
  (`KismetSystemLibrary.PrintString` "OnShowDualInventory")
  (bind _returnvalue (`|CreateWidget` "/Game/Survival/UI/Inventory/WBP_ChestInventory.WBP_ChestInventory_C" OwningController SourceInventory TargetInventory))
  (bind _output_get (set `self.ChestWidget` _returnvalue))
  (`UserWidget.AddToViewport` _output_get 0))

(fn `UserConstructionScript`)