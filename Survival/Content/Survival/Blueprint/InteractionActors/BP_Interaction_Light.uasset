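; BP_Interaction_Light is an interactable light actor that toggles on and off.
; The Interact event flips the IsOn variable, whose RepNotify function applies the state to the PointLight component.
; OnRep_IsOn activates or deactivates the light and also switches its color between white and black.
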(event `InteractInterface.Interact`
  (params (InstigatorController :type "Controller Object Reference"))
  (if (`self.IsOn`)
    (set `self.IsOn` false)
    (else
      (set `self.IsOn` true))))

(fn `OnRep_IsOn`
  (if (`self.IsOn`)
    (`ActorComponent.SetActive` (`self.PointLight`) true false)
    (`LightComponent.SetLightColor` (`self.PointLight`) (struct :`R` 1.0 :`G` 1.0 :`B` 1.0 :`A` 1.0) true)
    (else
      (`ActorComponent.SetActive` (`self.PointLight`) false false)
      (`LightComponent.SetLightColor` (`self.PointLight`) (struct :`A` 1.0) true))))

(fn `UserConstructionScript`
  (`parent.UserConstructionScript`))